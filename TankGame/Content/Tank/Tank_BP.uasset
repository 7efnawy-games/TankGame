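; Player-controllable tank Blueprint that routes input to its movement, aiming and camera components.
; BeginPlay initializes TankAiming with the barrel and turret, and TankMovement with the left and right tracks.
; Aim axes rotate an azimuth gimbal and spring arm, Fire calls TankAiming, and move axes pass turn, forward and backward intents to TankMovement.
; The construction script only prints a debug string.
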(event `self.ReceiveBeginPlay`
  (`TankAimingComponent.Initialize` (`self.TankAiming`) (`self.TankBarrel`) (`self.TankTurrent`))
  (`TankMovementComponent.Initialize` (`self.TankMovement`) (`self.LeftTrack`) (`self.RightTrack`)))

(event `InputAxis|AimAzimuth`
  (params (AxisValue :type "Float (single-precision)"))
  ;[1 1 1] AimInput Binding
  (`SceneComponent.K2_AddLocalRotation` (`self.AzimuthGimbal`) (`KismetMathLibrary.MakeRotator` 0.0 0.0 AxisValue) false false))

(event `InputAxis|AimElevation`
  (params (AxisValue :type "Float (single-precision)"))
  ;[1 1 1] AimInput Binding
  (`SceneComponent.K2_AddLocalRotation` (`self.SpringArm`) (`KismetMathLibrary.MakeRotator` 0.0 AxisValue) false false))

(event `InputAction|Fire`
  (params (Key :type "Key Structure"))
  ;[1 1 1] AimInput Binding
  (:`Pressed`
    (`TankAimingComponent.Fire` (`self.TankAiming`))))

(event `InputAxis|MoveLeft`
  (params (AxisValue :type "Float (single-precision)"))
  ;[1 1 1] TankMovement
  (`TankMovementComponent.IntendTurnLeft` (`self.TankMovement`) AxisValue))

(event `InputAxis|MoveRight`
  (params (AxisValue :type "Float (single-precision)"))
  ;[1 1 1] TankMovement
  (`TankMovementComponent.IntendTurnRight` (`self.TankMovement`) AxisValue))

(event `InputAxis|MoveForward`
  (params (AxisValue :type "Float (single-precision)"))
  ;[1 1 1] TankMovement
  (`TankMovementComponent.IntendMoveForward` (`self.TankMovement`) AxisValue))

(event `InputAxis|MoveBackwards`
  (params (AxisValue :type "Float (single-precision)"))
  ;[1 1 1] TankMovement
  (`TankMovementComponent.IntendMovebackward` (`self.TankMovement`) AxisValue))

(fn `UserConstructionScript`
  (`KismetSystemLibrary.PrintString` "JOE:ConstructCalledBLUEPRINT"))